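; Player-controlled world eater that flies with six-axis physics movement and absorbs meteorites.
; While Absorb is held, tagged objects in AbsorbRange receive meteorite gravity scaled by SizeScore, and meteorites entering AbsorbKillZone are eaten.
; Tick derives scale, camera distance, base speed and both sphere radii from SizeScore, which is not modified here.
; A cooldown-gated timeline dash boosts forward velocity and dampens turning, then sets movement speed to BaseSpeed.
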(event OnComponentBeginOverlap(AbsorbRange)
  (params (OtherActor :type Actor%20Object%20Reference) (OtherComp :type Primitive%20Component%20Object%20Reference) (OtherBodyIndex :type Integer) (bFromSweep :type Boolean) (SweepResult :type Hit%20Result%20Structure%20%28by%20ref%29))
  ;[1 1 1] Absorb Range Array
  (if (Components|ComponentHasTag OtherComp (Variables|Default|GetabsorbableTag))
    (Utilities|Array|Add (Variables|Default|GetobjectsInRange) OtherActor)
    (Development|PrintString (Utilities|GetDisplayName OtherActor))))

(event OnComponentEndOverlap(AbsorbRange)
  (params (OtherActor :type Actor%20Object%20Reference) (OtherComp :type Primitive%20Component%20Object%20Reference) (OtherBodyIndex :type Integer))
  ;[1 1 1] Absorb Range Array
  (if (Components|ComponentHasTag OtherComp (Variables|Default|GetabsorbableTag))
    (Utilities|Array|RemoveItem (Variables|Default|GetobjectsInRange) OtherActor)
    (Development|PrintString "removed")))

(event OnComponentBeginOverlap(AbsorbKillZone)
  (params (OtherActor :type Actor%20Object%20Reference) (OtherComp :type Primitive%20Component%20Object%20Reference) (OtherBodyIndex :type Integer) (bFromSweep :type Boolean) (SweepResult :type Hit%20Result%20Structure%20%28by%20ref%29))
  ;[1 1 1] Eating Section
  (if (Variables|Default|Getabsorbing)
    (bind _asmeteorite (Utilities|Casting|CastTometeorite OtherActor))
    (Default|Eaten _asmeteorite)))

(event EventTick
  (params (DeltaSeconds :type Float%20%28single-precision%29))
  ;[1 1 1] debug corner
  (Variables|Default|SetdeltaTime DeltaSeconds)
  (if (Variables|Default|Getdebug)
    (Development|PrintString "Hello"))
  (Variables|Default|SetDashElapsed (+ (Variables|Default|GetdeltaTime) (Variables|Default|GetDashElapsed)))
  (CallFunction|UpdateSize))

(event Input|ActionEvents|InputActionForwardDash
  ;[1 1 1] Charging Dash
  (:Pressed
    (if (> (Variables|Default|GetDashElapsed) (Variables|Default|GetDashTimeout))
      (Timeline|Short%20Dash PlayFromStart
        (:Update
          (Variables|Default|SetRotationMultiplier 0.1)
          (Variables|Default|SetMovementMultiplier 2e+02)
          (CallFunction|UpdateForwardMovement 1.0)
          (Variables|Default|SetDashElapsed 0.0))
        (:Finished
          (Variables|Default|SetRotationMultiplier 2.0)
          (Variables|Default|SetMovementMultiplier (Variables|Default|GetbaseSpeed)))))))

(event Input|AxisEvents|InputAxisMoveForward
  (params (AxisValue :type Float%20%28single-precision%29))
  ;[1 1 1] Forward Movement
  (CallFunction|UpdateForwardMovement AxisValue))

(event Input|AxisEvents|InputAxisMoveRight
  (params (AxisValue :type Float%20%28single-precision%29))
  ;[1 1 1] Right Movement
  (Physics|SetPhysicsLinearVelocity (Variables|Default|GetBodyMesh) (* (Math|Vector|GetRightVector (Transformation|GetActorRotation)) (* AxisValue (Variables|Default|GetMovementMultiplier))) true "None"))

(event Input|AxisEvents|InputAxisLookUp
  (params (AxisValue :type Float%20%28single-precision%29))
  ;[1 1 1] LookUp
  (Transformation|AddActorLocalRotation (Class|KismetMathLibrary|MakeRot (* AxisValue (Variables|Default|GetRotationMultiplier)) 0.0 0.0) false))

(event Input|AxisEvents|InputAxisTurn
  (params (AxisValue :type Float%20%28single-precision%29))
  (bind _rotationmultiplier (Variables|Default|GetRotationMultiplier))
  (bind _returnvalue (* AxisValue _rotationmultiplier))
  ;[1 1 1] Turn
  (Transformation|AddActorLocalRotation (Class|KismetMathLibrary|MakeRot 0.0 _returnvalue _returnvalue) false))

(event Input|AxisEvents|InputAxisAbsorb
  (params (AxisValue :type Float%20%28single-precision%29))
  ;[1 1 1] Absorb Activation
  (if (> AxisValue 0.0)
    (Variables|Default|Setabsorbing true)
    (for _array_element (Variables|Default|GetobjectsInRange)
      (bind _asmeteorite (Utilities|Casting|CastTometeorite _array_element))
      (Default|Gravity _asmeteorite (* AxisValue (* (Variables|Default|GetsizeScore) -1.0))))
    (else
      (Variables|Default|Setabsorbing false))))

(event Input|AxisEvents|InputAxisRiseAndFall
  (params (AxisValue :type Float%20%28single-precision%29))
  ;[1 1 1] Rise and Fall
  (Physics|SetPhysicsLinearVelocity (Variables|Default|GetBodyMesh) (* (Math|Vector|GetUpVector (Transformation|GetActorRotation)) (* AxisValue (Variables|Default|GetMovementMultiplier))) true "None"))

(fn ConstructionScript)

(fn UpdateForwardMovement
  (params (LocalAxis :type Float%20%28single-precision%29))
  (Physics|SetPhysicsLinearVelocity (Variables|Default|GetBodyMesh) (* (Math|Vector|GetForwardVector (Transformation|GetActorRotation)) (* LocalAxis (Variables|Default|GetMovementMultiplier))) true "None")
  (return))

(fn UpdateSize
  (bind _sizescore (Variables|Default|GetsizeScore))
  (bind _returnvalue (/ _sizescore 1e+02))
  (Transformation|SetActorScale3D (Math|Vector|MakeVector _returnvalue _returnvalue _returnvalue))
  (Variables|/Script/Engine.SpringArmComponent|SetTargetArmLength (Variables|Default|GetCameraArm) (* _returnvalue 5e+02))
  (Variables|Default|SetbaseSpeed (* _returnvalue 3e+01))
  (Components|Sphere|SetSphereRadius (Variables|Default|GetAbsorbKillZone) (* _returnvalue 64.0) true)
  (Components|Sphere|SetSphereRadius (Variables|Default|GetAbsorbRange) (* _returnvalue 3.6e+02) true)
  (return))