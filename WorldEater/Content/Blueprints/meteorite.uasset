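; Meteorite that the world-eater player (BP_WorldEater2) can consume to increase its SizeScore.
; Gravity adds physics velocity along the player-to-meteorite direction, scaled by Force divided by SizeScore, so larger meteorites react less.
; Eaten adds the meteorite's SizeScore to the player's, prints a debug score, destroys the actor and spawns an explosion at its location.
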(fn ConstructionScript)

(fn Gravity
  (params (Force :type Float%20%28single-precision%29))
  (Physics|SetPhysicsLinearVelocity (* (Class|KismetMathLibrary|GetDirectionVector (Transformation|GetActorLocation (Game|Player|GetPlayerPawn 0)) (Transformation|GetActorLocation)) (/ Force (Variables|Default|GetsizeScore))) true "None"))

(fn Eaten
  (bind _asbp_world_eater_2 (Utilities|Casting|CastToBP_WorldEater2 (Game|Player|GetPlayerPawn 0)))
  (Variables|/Game/Blueprints/BP_WorldEater2.BP_WorldEater2_C|SetsizeScore _asbp_world_eater_2 (+ (Variables|Default|GetsizeScore) (Variables|/Game/Blueprints/BP_WorldEater2.BP_WorldEater2_C|GetsizeScore _asbp_world_eater_2)))
  (Development|PrintString (Utilities|String|ToString(Float) (+ (Variables|Default|GetsizeScore) (Variables|/Game/Blueprints/BP_WorldEater2.BP_WorldEater2_C|GetsizeScore _asbp_world_eater_2))))
  (Actor|DestroyActor)
  (Effects|SpawnEmitteratLocation "/Game/Particles/P_Explosion.P_Explosion" (Transformation|GetActorLocation)))