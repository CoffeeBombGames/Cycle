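; BP_WorldEater is a player-controlled actor that flies by physics and carries an unfinished forward dash.
; Move axes add velocity to BodyMesh along the actor's forward and right vectors.
; Look axes apply local rotations, with Turn adding equal roll to yaw.
; ForwardDash starts a Tick-driven timer; later presses past the timeout only reset it and print a message, as no dash impulse exists.
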(event EventTick
  (params (DeltaSeconds :type Float%20%28single-precision%29))
  ;[1 1 1] Forward Dash
  (if (Variables|Default|GettryingDash)
    (Variables|Default|SetDashElapsed (+ DeltaSeconds (Variables|Default|GetDashElapsed)))))

(event Input|ActionEvents|InputActionForwardDash
  ;[1 1 1] Forward Dash
  (:Pressed
    (if (Variables|Default|GettryingDash)
      (if (not (<= (Variables|Default|GetDashElapsed) (Variables|Default|GetDashTimeout)))
        (Variables|Default|SetDashElapsed 0.0)
        (Development|PrintString "Dash timed out."))
      (else
        (Variables|Default|SettryingDash true)))))

(event Input|AxisEvents|InputAxisMoveForward
  (params (AxisValue :type Float%20%28single-precision%29))
  ;[1 1 1] Forward Movement
  (Physics|SetPhysicsLinearVelocity (Variables|Default|GetBodyMesh) (* (Math|Vector|GetForwardVector (Transformation|GetActorRotation)) (* AxisValue 5e+01)) true "None"))

(event Input|AxisEvents|InputAxisMoveRight
  (params (AxisValue :type Float%20%28single-precision%29))
  ;[1 1 1] Right Movement
  (Physics|SetPhysicsLinearVelocity (Variables|Default|GetBodyMesh) (* (Math|Vector|GetRightVector (Transformation|GetActorRotation)) (* AxisValue 5e+01)) true "None"))

(event Input|AxisEvents|InputAxisLookUp
  (params (AxisValue :type Float%20%28single-precision%29))
  ;[1 1 1] LookUp
  (Transformation|AddActorLocalRotation (Class|KismetMathLibrary|MakeRot (/ AxisValue 2.5) 0.0 0.0) false))

(event Input|AxisEvents|InputAxisTurn
  (params (AxisValue :type Float%20%28single-precision%29))
  (bind _returnvalue (/ AxisValue 2.5))
  ;[1 1 1] Turn
  (Transformation|AddActorLocalRotation (Class|KismetMathLibrary|MakeRot 0.0 _returnvalue _returnvalue) false))

(fn ConstructionScript)